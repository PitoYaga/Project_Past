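; BP_Studio is an item inspection actor that displays a chosen mesh while the player examines it.
; Inspect assigns the mesh to its StaticMesh component, shows a WB_ItemInfo widget, and moves input from the player to itself.
; Pressing Interact ends inspection by returning input to the player and removing the widget, leaving the mesh assigned.
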(event `/Game/Interact/BP_InteractInterface.Inspect`
  (params (Player :type "/Game/FirstPerson/Blueprints/BP_FirstPersonCharacter Object Reference") (ItemToFocus :type "StaticMesh Object Reference") (ItemName :type Text) (ItemDescription :type Text))
  (bind _returnvalue (`GameplayStatics.GetPlayerController` 0))
  (set `self.Player` Player)
  (`StaticMeshComponent.SetStaticMesh` (`self.StaticMesh`) ItemToFocus)
  (bind _returnvalue_2 (`|CreateWidget` "/Game/Interact/Inspect/WB_ItemInfo.WB_ItemInfo_C"))
  (bind _output_get (set `self.ItemDetailWidget` _returnvalue_2))
  (`UserWidget.AddToViewport` _output_get 0)
  (`self.DisableInput` (`self.Player`) _returnvalue)
  (`self.EnableInput` _returnvalue))

(event `InputAction|Interact`
  (params (Key :type "Key Structure"))
  (bind _returnvalue (`GameplayStatics.GetPlayerController` 0))
  (:`Pressed`
    (`self.DisableInput` _returnvalue)
    (`self.EnableInput` (`self.Player`) _returnvalue)
    (`Widget.RemoveFromParent` (`self.ItemDetailWidget`))
    (set `self.ItemDetailWidget` null)))

(fn `UserConstructionScript`)