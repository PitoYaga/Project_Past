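; BP_InspectableObject is an interactable world item that the player can inspect.
; Its InteractRadius overlap creates and shows a WB_Inspect_UI prompt for the first-person character, removing it on exit, while trace events toggle the prompt's border highlight.
; Interact spawns a BP_Studio far away from the origin and passes it the player, item mesh, name and description for inspection.
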(event `self.InteractRadius.OnComponentBeginOverlap`
  (params (OverlappedComponent :type "PrimitiveComponent Object Reference") (OtherActor :type "Actor Object Reference") (OtherComp :type "PrimitiveComponent Object Reference") (OtherBodyIndex :type Integer) (bFromSweep :type Boolean) (SweepResult :type "HitResult Structure (by ref)"))
  (bind _widget (`self.Widget`))
  (cast `/Game/FirstPerson/Blueprints/BP_FirstPersonCharacter` OtherActor)
  (bind _returnvalue (`|CreateWidget` "/Game/Interactable_Objects/Inspect/WB_Inspect_UI.WB_Inspect_UI_C"))
  (bind _output_get (set `self.InteractionWidget` _returnvalue))
  (`WidgetComponent.SetWidget` _widget _output_get)
  (`SceneComponent.SetVisibility` _widget true false))

(event `self.InteractRadius.OnComponentEndOverlap`
  (params (OverlappedComponent :type "PrimitiveComponent Object Reference") (OtherActor :type "Actor Object Reference") (OtherComp :type "PrimitiveComponent Object Reference") (OtherBodyIndex :type Integer))
  (cast `/Game/FirstPerson/Blueprints/BP_FirstPersonCharacter` OtherActor)
  (`Widget.RemoveFromParent` (`self.InteractionWidget`))
  (set `self.InteractionWidget` null)
  (`SceneComponent.SetVisibility` (`self.Widget`) false false))

(event `/Game/Interactable_Objects/BP_InteractInterface.CanRecieveTrace`
  (params (CanInteract :type Boolean))
  (if CanInteract
    (bind _interactionwidget (`self.InteractionWidget`)
      (:`then`
        (`Widget.SetRenderOpacity` (`/Game/Interactable_Objects/Inspect/WB_Inspect_UI.InteractionBorder` _interactionwidget) 1.0))
      (:`else`))
    (else
      (bind _interactionwidget_2 (`self.InteractionWidget`)
        (:`then`
          (`Widget.SetRenderOpacity` (`/Game/Interactable_Objects/Inspect/WB_Inspect_UI.InteractionBorder` _interactionwidget_2) 0.0))
        (:`else`)))))

(event `/Game/Interactable_Objects/BP_InteractInterface.Interact`
  (params (Player :type "/Game/FirstPerson/Blueprints/BP_FirstPersonCharacter Object Reference"))
  (bind _returnvalue (`|SpawnActorFromClass` "/Game/Interactable_Objects/Inspect/BP_Studio.BP_Studio_C" (`KismetMathLibrary.MakeTransform` (1000000000.0 0.0 0.0)) "Undefined" "OverrideRootScale" null null))
  (message `/Game/Interactable_Objects/BP_InteractInterface.Inspect` _returnvalue Player (`StaticMeshComponent.StaticMesh` (`self.Item`)) (`self.ItemName`) (`self.ItemDescription`)))

(fn `UserConstructionScript`)