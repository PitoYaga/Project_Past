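; BP_Studio is an item inspection actor that shows a given mesh for the player to rotate and examine.
; Inspect sets the mesh, adds a WB_ItemInfo widget with name and description, and moves input from the player to this actor.
; Left-mouse drag or the movement axes rotate the mesh in pitch and yaw via combined world rotations.
; Pressing Interact restores player input, removes the widget and destroys the actor.
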(event `/Game/Interactable_Objects/BP_InteractInterface.Inspect`
  (params (Player :type "/Game/FirstPerson/Blueprints/BP_FirstPersonCharacter Object Reference") (ItemToFocus :type "StaticMesh Object Reference") (ItemName :type Text) (ItemDescription :type Text))
  (bind _returnvalue (`GameplayStatics.GetPlayerController` 0))
  ;[1 1 1] Inspect_Start
  (set `self.Player` Player)
  (`StaticMeshComponent.SetStaticMesh` (`self.StaticMesh`) ItemToFocus)
  (bind _returnvalue_2 (`|CreateWidget` "/Game/Interactable_Objects/Inspect/WB_ItemInfo.WB_ItemInfo_C" null ItemName ItemDescription))
  (bind _output_get (set `self.ItemDetailWidget` _returnvalue_2))
  (`UserWidget.AddToViewport` _output_get 0)
  (`self.DisableInput` (`self.Player`) _returnvalue)
  (`self.EnableInput` _returnvalue))

(event `InputAction|Interact`
  (params (Key :type "Key Structure"))
  (bind _returnvalue (`GameplayStatics.GetPlayerController` 0))
  ;[1 1 1] Inspect_End
  (:`Pressed`
    (`self.DisableInput` _returnvalue)
    (`self.EnableInput` (`self.Player`) _returnvalue)
    (`Widget.RemoveFromParent` (`self.ItemDetailWidget`))
    (set `self.ItemDetailWidget` null)
    (`self.K2_DestroyActor` self)))

(event `Key|LeftMouseButton`
  (params (Key :type "Key Structure"))
  ;[1 1 1] Rotate_Object
  ;;[1 1 1] Mouse_Rotation
  (:`Pressed`
    (set `self.CanRotate` true))
  (:`Released`
    (set `self.CanRotate` false)))

(event `InputAxis|MoveForward`
  (params (AxisValue :type "Float (single-precision)"))
  ;[1 1 1] Rotate_Object
  ;;[1 1 1] Keyboard_Rotation
  (if (!= AxisValue 0.0)
    (`SceneComponent.K2_SetWorldRotation` (`self.StaticMesh`) (`KismetMathLibrary.ComposeRotators` (`SceneComponent.K2_GetComponentRotation` (`self.StaticMesh`)) (`KismetMathLibrary.MakeRotator` 0.0 (* AxisValue -2.0))) false false)))

(event `InputAxisKey|MouseX`
  (params (AxisValue :type "Float (single-precision)"))
  ;[1 1 1] Rotate_Object
  ;;[1 1 1] Mouse_Rotation
  (if (`self.CanRotate`)
    (`SceneComponent.K2_SetWorldRotation` (`self.StaticMesh`) (`KismetMathLibrary.ComposeRotators` (`SceneComponent.K2_GetComponentRotation` (`self.StaticMesh`)) (`KismetMathLibrary.MakeRotator` 0.0 0.0 (* AxisValue -2.0))) false false)))

(event `InputAxis|MoveRight`
  (params (AxisValue :type "Float (single-precision)"))
  ;[1 1 1] Rotate_Object
  ;;[1 1 1] Keyboard_Rotation
  (if (!= AxisValue 0.0)
    (`SceneComponent.K2_SetWorldRotation` (`self.StaticMesh`) (`KismetMathLibrary.ComposeRotators` (`SceneComponent.K2_GetComponentRotation` (`self.StaticMesh`)) (`KismetMathLibrary.MakeRotator` 0.0 0.0 (* AxisValue -2.0))) false false)))

(event `InputAxisKey|MouseY`
  (params (AxisValue :type "Float (single-precision)"))
  ;[1 1 1] Rotate_Object
  ;;[1 1 1] Mouse_Rotation
  (if (`self.CanRotate`)
    (`SceneComponent.K2_SetWorldRotation` (`self.StaticMesh`) (`KismetMathLibrary.ComposeRotators` (`SceneComponent.K2_GetComponentRotation` (`self.StaticMesh`)) (`KismetMathLibrary.MakeRotator` 0.0 (* AxisValue -2.0))) false false)))

(fn `UserConstructionScript`)