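; BP_Partner is a character that walks through an ordered list of waypoint actors from BeginPlay.
; PathFind advances the index and restores walk speed, feeding a looping AI MoveTo.
; On each arrival, talk and animation functions match the index against their location lists, print placeholder messages and can zero walk speed.
; That stop is immediately overwritten while waypoints remain, and both functions compare against AnimIndex.
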(event `MoveToLocation`
  (bind _locations (`self.PathFind` :!label _label))
  (`|AIMoveTo` self _locations null
    (:`OnSuccess`
      (`self.TalkAtLocation` (`self.TalkLocation`) (`self.TalkWalkSpeed`))
      (`self.PlayAnimAtLocation` (`self.AnimLocation`) (`self.AnimWalkSpeed`))
      (goto _label))))

(event `self.ReceiveBeginPlay`
  (`self.MoveToLocation`))

(fn `PathFind`
  (returns (Locations :type "Vector Structure"))
  (bind _pathlocs (`self.PathLocs`))
  (if (not (>= (`self.PathLocIndex`) (- (`KismetArrayLibrary.Array_Length` _pathlocs) 1)))
    (`/Engine/EditorBlueprintResources/StandardMacros.IncrementInt` (`self.PathLocIndex`)
      (:`  `
        (set `CharacterMovementComponent.MaxWalkSpeed` (`self.WalkSpeed`) (`self.CharacterMovement`))
        (return (`self.K2_GetActorLocation` (`|GetArrayItem` _pathlocs (`self.PathLocIndex`))))))))

(fn `PlayAnimAtLocation`
  (params (AnimLocation :type "Array of Integer") (AnimWalkSpeed :type "Array of Float (double-precision)"))
  (for _array_element AnimLocation
    (if (== _array_element (`self.PathLocIndex`))
      (`KismetSystemLibrary.PrintString` "Do a flip")
      (for (_ _array_index) AnimWalkSpeed :!label _label
        (if (== _array_index (`self.AnimIndex`))
          (set `CharacterMovementComponent.MaxWalkSpeed` 0.0 (`self.CharacterMovement`))
          (`/Engine/EditorBlueprintResources/StandardMacros.IncrementInt` (`self.AnimIndex`)
            (:`  `
              (`KismetSystemLibrary.PrintString` "Hello")
              (break)))
          (else
            (goto _label)))))))

(fn `TalkAtLocation`
  (params (TalkLocation :type "Array of Integer") (TalkWalkSpeed :type "Array of Float (double-precision)"))
  (for _array_element TalkLocation
    (if (== _array_element (`self.PathLocIndex`))
      (`KismetSystemLibrary.PrintString` "play sound")
      (for (_ _array_index) TalkWalkSpeed
        (if (== _array_index (`self.AnimIndex`))
          (set `CharacterMovementComponent.MaxWalkSpeed` 0.0 (`self.CharacterMovement`))
          (`/Engine/EditorBlueprintResources/StandardMacros.IncrementInt` (`self.TalkIndex`)
            (:`  `
              (break)))))
      (else
        (`KismetSystemLibrary.PrintString` "continue  walking")))))

(fn `UserConstructionScript`)